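; Camera actor that drives a toggleable Voronoi split screen through a scene capture component.
; Each tick it updates the capture FOV and, while split screen is active, either creates the capture widget or runs the dynamic split-screen logic, both defined outside this graph except widget setup.
; Setup adds a widget showing the capture material to the viewport and assigns the capture's render target.
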(event EventBeginPlay
  (Variables|Default|SetPassedFOV (Variables|Default|GetFOV)))

(event Collision|EventActorBeginOverlap
  (params (OtherActor :type Actor%20Object%20Reference)))

(event EventTick
  (params (DeltaSeconds :type Float%20%28single-precision%29))
  (Class|VoronoiCameraActor|UpdatingFOV (Variables|Default|GetFOV) (Variables|Default|GetPassedFOV) (Variables|Default|GetSceneCaptureComponent2D))
  (if (Variables|Default|GetActivateVoronoiSplitScreen)
    (if (Variables|Default|GetIsWidgetReady)
      (Class|VoronoiCameraActor|ActivateDynamicSplitScreen)
      (else
        (CallFunction|ActivateVoronoiWidget)))
    (else
      (Variables|Default|SetIsWidgetReady false))))

(fn ConstructionScript)

(fn ActivateVoronoiWidget
  (bind _returnvalue (UserInterface|CreateWidget "/Game/Interface/VoronoiInterface/BP_CaptureWidget.BP_CaptureWidget_C"))
  (Variables|/Game/Interface/VoronoiInterface/BP_CaptureWidget.BP_CaptureWidget_C|SetCapturedMaterial _returnvalue "/Game/Materials/VoronoiMaterials/M_CaptureMaterial_Inst.M_CaptureMaterial_Inst")
  (UserInterface|Viewport|AddtoViewport _returnvalue 0)
  (Variables|/Script/Engine.SceneCaptureComponent2D|SetTextureTarget (Variables|Default|GetSceneCaptureComponent2D) (Variables|Default|GetCaptureTextureTarget))
  (Variables|Default|SetIsWidgetReady true))