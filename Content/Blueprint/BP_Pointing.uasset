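; BP_Pointing is a pointer actor built to bob up and down and turn its static mesh toward the player holding the dustpan.
; BeginPlay caches the CharacterManager and the starting location.
; A ping-pong time value would lerp the actor along its up vector while RotateToPlayer sets the mesh's look-at yaw.
; That movement chain is disconnected from the empty Tick, so it never runs.
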(event EventBeginPlay
  (bind _outactors (Actor|GetAllActorsOfClass "/Script/Twaliens.CharacterManager"))
  (Variables|Default|SetCharacterManager (Utilities|Array|Get(acopy) _outactors))
  (Variables|Default|SetDefaultLocation (Transformation|GetActorLocation)))

(event Collision|EventActorBeginOverlap
  (params (OtherActor :type Actor%20Object%20Reference)))

(event EventTick
  (params (DeltaSeconds :type Float%20%28single-precision%29)))

(fn ConstructionScript)

(fn RotatetoPlayer
  (Transformation|SetWorldRotation (Variables|Default|GetStaticMesh) (Math|Rotator|MakeRotator -9e+01 0.0 (.yaw (Math|Rotator|FindLookatRotation (Transformation|GetWorldLocation (Variables|Default|GetStaticMesh)) (Transformation|GetActorLocation (Class|CharacterManager|GetPlayerwithDustpan (Variables|Default|GetCharacterManager)))))) false false))

(fn GetMultplier
  (if (>= (Variables|Default|GetTime) 1.0)
    (Variables|Default|SetMultiplier -1.0)
    (elif (<= (Variables|Default|GetTime) 0.0)
      (Variables|Default|SetMultiplier 1.0))))

(fn SetAlpha
  (params (A :type Float%20%28single-precision%29))
  (bind _output_get (Variables|Default|SetTime (+ (Variables|Default|GetTime) (* (* A 1.25) (Variables|Default|GetMultiplier)))))
  (return _output_get))