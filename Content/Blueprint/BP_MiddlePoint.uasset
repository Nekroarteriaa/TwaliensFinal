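; BP_MiddlePoint is an arrow indicator between the two players that warns of an upcoming switch.
; Each tick it moves to their midpoint, turns along their line, and scales both widgets and arrow material tiling by distance.
; A looping timer raises the arrows' Gradient once player 0's remaining switch time is within TimeToShowArrows, then reveals a particle system.
; Gradient and particles reset outside that window or when that player is dead.
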(event EventBeginPlay
  (Utilities|Time|SetTimerbyFunctionName 0 "ShowArrows" 0.5 true))

(event Collision|EventActorBeginOverlap
  (params (OtherActor :type Actor%20Object%20Reference)))

(event EventTick
  (params (DeltaSeconds :type Float%20%28single-precision%29))
  (CallFunction|ActualizeMiddlePoint)
  (CallFunction|GettheRotation)
  (CallFunction|ScaletheMaterial))

(fn ConstructionScript
  (bind _returnvalue (Rendering|Material|CreateDynamicMaterialInstance (Variables|Default|GetArrow1) 0 0 "None" :!class /Script/Engine.PrimitiveComponent))
  (Variables|Default|SetArrowMaterial _returnvalue)
  (bind _returnvalue_2 (Rendering|Material|CreateDynamicMaterialInstance (Variables|Default|GetArrow2) 0 0 "None" :!class /Script/Engine.PrimitiveComponent))
  (Variables|Default|SetArrowMaterial2 _returnvalue_2))

(fn ScaletothePlayers)

(fn ActualizeMiddlePoint
  (bind _returnvalue (Game|GetPlayerCharacter 1))
  (bind _returnvalue_2 (Game|GetPlayerCharacter 0))
  (bind _mesh (Variables|/Script/Engine.Character|GetMesh _returnvalue))
  (bind _mesh_2 (Variables|/Script/Engine.Character|GetMesh _returnvalue_2))
  (bind _returnvalue_3 (Transformation|GetWorldLocation _mesh))
  (bind _returnvalue_4 (Transformation|GetWorldLocation _mesh_2))
  (Transformation|SetWorldLocation (Variables|Default|GetDefaultSceneRoot) (Math|Vector|MakeVector (/ (+ (.x _returnvalue_3) (.x _returnvalue_4)) 2.0) (/ (+ (.y _returnvalue_3) (.y _returnvalue_4)) 2.0) (.z _returnvalue_3)) false false))

(fn GettheRotation
  (bind _returnvalue (Game|GetPlayerCharacter 1))
  (bind _self self)
  (bind _defaultsceneroot (Variables|Default|GetDefaultSceneRoot _self))
  (bind _mesh (Variables|/Script/Engine.Character|GetMesh _returnvalue))
  (bind _returnvalue_2 (Transformation|GetWorldLocation _mesh))
  (bind _returnvalue_3 (Transformation|GetWorldLocation _defaultsceneroot))
  (bind _returnvalue_4 (Math|Rotator|FindLookatRotation _returnvalue_2 _returnvalue_3))
  (Transformation|SetWorldRotation _defaultsceneroot (Math|Rotator|MakeRotator (.roll _returnvalue_4) (.pitch (Transformation|GetWorldRotation _defaultsceneroot)) (.yaw _returnvalue_4)) false false))

(fn ScaletheMaterial
  (bind _returnvalue (Game|GetPlayerCharacter 1))
  (bind _self self)
  (bind _widget (Variables|Default|GetWidget))
  (bind _widget1 (Variables|Default|GetWidget1))
  (bind _returnvalue_2 (Transformation|GetDistanceTo _returnvalue _self))
  (bind _returnvalue_3 (Transformation|GetWorldScale _widget1))
  (bind _returnvalue_4 (Transformation|GetWorldScale _widget))
  (bind _returnvalue_5 (- _returnvalue_2 2e+02))
  (bind _returnvalue_6 (* 0.01 _returnvalue_5))
  (bind _returnvalue_7 (* _returnvalue_6 2.0))
  (Transformation|SetWorldScale3D _widget1 (Math|Vector|MakeVector _returnvalue_6 (.y _returnvalue_3) (.z _returnvalue_3)))
  (Transformation|SetWorldScale3D _widget (Math|Vector|MakeVector _returnvalue_6 (.y _returnvalue_4) (.z _returnvalue_4)))
  (Rendering|Material|SetScalarParameterValue (Variables|Default|GetArrowMaterial) "TilingValue" _returnvalue_7 :!class /Script/Engine.MaterialInstanceDynamic)
  (Rendering|Material|SetScalarParameterValue (Variables|Default|GetArrowMaterial2) "TilingValue" _returnvalue_7 :!class /Script/Engine.MaterialInstanceDynamic))

(fn ShowArrows
  (bind _arrowmaterial (Variables|Default|GetArrowMaterial))
  (bind _asbp_twalien_0 (Utilities|Casting|CastToBP_Twalien_0 (Game|GetPlayerCharacter 0)))
  (if (<= (Class|CharacterManager|GetRemainingSwitchTime (Variables|/Game/Characters/Player/BP_Twalien_0.BP_Twalien_0_C|GetCharacterManager _asbp_twalien_0)) (Variables|Default|GetTimeToShowArrows))
    (bind _returnvalue (Rendering|Material|GetScalarParameterValue _arrowmaterial "Gradient" :!class /Script/Engine.MaterialInstanceDynamic))
    (Rendering|Material|SetScalarParameterValue _arrowmaterial "Gradient" (+ _returnvalue 0.05) :!class /Script/Engine.MaterialInstanceDynamic)
    (Rendering|Material|SetScalarParameterValue (Variables|Default|GetArrowMaterial2) "Gradient" (+ _returnvalue 0.05) :!class /Script/Engine.MaterialInstanceDynamic)
    (if (Variables|/Script/Twaliens.Twalien|GetIsDead _asbp_twalien_0)
      (Rendering|Material|SetScalarParameterValue (Variables|Default|GetArrowMaterial) "Gradient" 0.0 :!class /Script/Engine.MaterialInstanceDynamic :!label _label)
      (Rendering|Material|SetScalarParameterValue (Variables|Default|GetArrowMaterial2) "Gradient" 0.0 :!class /Script/Engine.MaterialInstanceDynamic)
      (Rendering|SetVisibility (Variables|Default|GetParticleSystem) false false)
      (elif (>= (+ _returnvalue 0.05) 0.5)
        (Rendering|SetVisibility (Variables|Default|GetParticleSystem) true false)))
    (else
      (goto _label))))