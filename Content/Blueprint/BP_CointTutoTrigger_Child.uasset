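; Child of a coin tutorial trigger that watches the Ammo actors inside its volume and removes itself once none remain.
; Overlap events add and remove Ammo in an array, which Tick polls through a 0.2-second Delay.
; When the array is empty, it resets the Spawner's spawned-enemy count and destroys itself.
; End overlap also hides the Pointing actor when the dustpan-holding player leaves.
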(event EventBeginPlay
  (|CallParentFunction) ; This node is disabled and will not be called.\nDrag off pins to build functionality.
)

(event Collision|EventActorBeginOverlap
  (params (OtherActor :type Actor%20Object%20Reference))
  (|CallParentFunction OtherActor)
  (bind _asammo (Utilities|Casting|CastToAmmo OtherActor))
  (Utilities|Array|Add (Variables|Default|GetAmmo) _asammo))

(event EventTick
  (params (DeltaSeconds :type Float%20%28single-precision%29))
  (|CallParentFunction DeltaSeconds)
  (Utilities|FlowControl|Delay 0.2)
  (if (<= (Utilities|Array|Length (Variables|Default|GetAmmo)) 0)
    (Variables|/Game/Characters/Objects/BP_EnemySpawner_2.BP_EnemySpawner_2_C|SetEnemiesSpawned (Variables|Default|GetSpawner) 0)
    (Actor|DestroyActor)))

(event Collision|EventActorEndOverlap
  (params (OtherActor :type Actor%20Object%20Reference))
  (bind _pointing (Variables|Default|GetPointing))
  (bind _charactermanager (Variables|Default|GetCharacterManager))
  (bind _returnvalue (Class|CharacterManager|GetPlayerwithDustpan _charactermanager))
  (bind _asammo (Utilities|Casting|CastToAmmo OtherActor)
    (:then
      (Utilities|Array|RemoveItem (Variables|Default|GetAmmo) _asammo))
    (:CastFailed
      _))
  (Utilities|IsValid _pointing
    (:Is%20Valid
      (Utilities|IsValid _returnvalue
        (:Is%20Valid
          (if (== OtherActor _returnvalue)
            (Rendering|SetActorHiddenInGame _pointing true)))))))

(fn ConstructionScript
  (|CallParentFunction))