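; BP_Rock is a rock actor that moves with sound once its linked EnemySpawner is destroyed.
; The spawner's OnDestroyed event sets an ActivateAnimation flag, which Tick polls to play FMOD audio, cache the current location and start a timeline.
; The timeline adds its Movement offset to that cached location without sweeping and clears the flag on update.
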(event OnDestroyed(EnemySpawner)
  (params (DestroyedActor :type Actor%20Object%20Reference))
  (Variables|Default|SetActivateAnimation true))

(event EventBeginPlay)

(event EventTick
  (params (DeltaSeconds :type Float%20%28single-precision%29))
  (if (Variables|Default|GetActivateAnimation)
    (Class|FMODAudioComponent|Play (Variables|Default|GetFMODAudio))
    (Variables|Default|SetLocInicial (Transformation|GetActorLocation))
    (bind _movement (Timeline|Timeline_0 Play)
      (:Update
        (Transformation|SetActorLocation (+ _movement (Variables|Default|GetLocInicial)) false false)
        (Variables|Default|SetActivateAnimation false)))))

(fn ConstructionScript)