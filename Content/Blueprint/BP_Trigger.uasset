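; BP_Trigger is a trigger volume that shows a Pointing actor while the player holding the dustpan is inside it.
; Shortly after BeginPlay it switches its collision component to the Trigger profile.
; On overlap begin it unhides Pointing only if the actor matches the CharacterManager's player with the dustpan.
; On overlap end it hides Pointing again, whichever actor leaves.
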(event EventBeginPlay
  (Utilities|FlowControl|Delay 0.2)
  (Collision|SetCollisionProfileName (Variables|Default|GetCollisionComponent) "Trigger" :!class /Script/Engine.PrimitiveComponent))

(event Collision|EventActorBeginOverlap
  (params (OtherActor :type Actor%20Object%20Reference))
  (bind _charactermanager (Variables|Default|GetCharacterManager))
  (bind _pointing (Variables|Default|GetPointing))
  (bind _returnvalue (Class|CharacterManager|GetPlayerwithDustpan _charactermanager))
  (Utilities|IsValid _returnvalue
    (:Is%20Valid
      (if (== OtherActor _returnvalue)
        (Utilities|IsValid _pointing
          (:Is%20Valid
            (Rendering|SetActorHiddenInGame _pointing false)))))))

(event EventTick
  (params (DeltaSeconds :type Float%20%28single-precision%29)))

(event Collision|EventActorEndOverlap
  (params (OtherActor :type Actor%20Object%20Reference))
  (bind _pointing (Variables|Default|GetPointing))
  (Utilities|IsValid _pointing
    (:Is%20Valid
      (Rendering|SetActorHiddenInGame _pointing true))))

(fn ConstructionScript)