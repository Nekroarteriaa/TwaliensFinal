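; Twalien player character Blueprint for a two-player game, with a pause-menu input and a world-space compass oriented by the other player's position.
; Tick rotates the compass along the look-at direction from the other character's mesh to the widget.
; BeginPlay caches the CharacterManager and, after a short delay, assigns a per-player compass material.
; Switch-timer compass scaling and recoloring functions exist, but their EventGraph call is disconnected.
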(event EventBeginPlay
  (bind _outactors (Actor|GetAllActorsOfClass "/Script/Twaliens.CharacterManager"))
  (for _array_element _outactors
    (Variables|Default|SetCharacterManager _array_element)
    (Utilities|FlowControl|Delay 0.05)
    (CallFunction|CompasColorChangeIni)))

(event Collision|EventActorBeginOverlap
  (params (OtherActor :type Actor%20Object%20Reference)))

(event EventTick
  (params (DeltaSeconds :type Float%20%28single-precision%29))
  (CallFunction|CompassRefresh))

(event Input|ActionEvents|InputActionPause
  (params (Key :type Key%20Structure))
  (bind _returnvalue (Game|GetPlayerController 0))
  ;[1 1 1] Menu Pausa
  (:Pressed
    (if (not (Variables|Default|GetIsGamePaused))
      (Game|SetGamePaused true)
      (bind _returnvalue_2 (UserInterface|CreateWidget "/Game/Interface/MenuPausa.MenuPausa_C" _returnvalue))
      (UserInterface|Viewport|AddtoViewport _returnvalue_2 0)
      (Input|SetInputModeUIOnly _returnvalue 0 "DoNotLock")
      (Variables|/Script/Engine.PlayerController|SetbShowMouseCursor _returnvalue true))))

(fn ConstructionScript)

(fn CompassRefresh
  (bind _returnvalue (Game|GetPlayerCharacter 1))
  (bind _returnvalue_2 (Game|GetPlayerCharacter 0))
  (bind _widgetcompass (Variables|Default|GetWidgetCompass))
  (bind _returnvalue_3 (Transformation|GetWorldLocation _widgetcompass))
  (bind _returnvalue_4 (Transformation|GetWorldRotation _widgetcompass))
  (bind _mesh (Variables|/Script/Engine.Character|GetMesh _returnvalue))
  (bind _mesh_2 (Variables|/Script/Engine.Character|GetMesh _returnvalue_2))
  (bind _returnvalue_5 (Transformation|GetWorldLocation _mesh))
  (bind _returnvalue_6 (Transformation|GetWorldLocation _mesh_2))
  (bind _returnvalue_7 (Math|Rotator|FindLookatRotation _returnvalue_6 _returnvalue_3))
  (bind _returnvalue_8 (Math|Rotator|FindLookatRotation _returnvalue_5 _returnvalue_3))
  (if (== self _returnvalue_2)
    (bind _output_get (Variables|Default|SetCompassRotation (.yaw _returnvalue_8)))
    (Transformation|SetWorldRotation _widgetcompass (Math|Rotator|MakeRotator (.roll _returnvalue_8) (.pitch _returnvalue_4) _output_get) false false)
    (else
      (bind _output_get_2 (Variables|Default|SetCompassRotation (.yaw _returnvalue_7)))
      (Transformation|SetWorldRotation _widgetcompass (Math|Rotator|MakeRotator (.roll _returnvalue_7) (.pitch _returnvalue_4) _output_get_2) false false))))

(fn CompassTimeSize
  (bind _charactermanager (Variables|Default|GetCharacterManager))
  (bind _widgetcompass (Variables|Default|GetWidgetCompass))
  (bind _compastimetogrowstart (Variables|Default|GetCompasTimeToGrowStart))
  (bind _returnvalue (Transformation|GetWorldScale _widgetcompass))
  (bind _returnvalue_2 (Class|CharacterManager|GetRemainingSwitchTime _charactermanager))
  (bind _returnvalue_3 (Math|Float|Max(Float) _returnvalue_2 0.0001))
  (bind _returnvalue_4 (/ 0.05 _returnvalue_3))
  (bind _returnvalue_5 (+ (.y _returnvalue) _returnvalue_4))
  (bind _returnvalue_6 (Math|Float|Min(Float) _returnvalue_5 2.0))
  (if (and (> _returnvalue_2 _compastimetogrowstart) (< _returnvalue_2 (Variables|Default|GetCompassTimeToChangeColors)))
    (Variables|Default|Setflag true)
    (CallFunction|CompasRecolor :!label _label)
    (elif (> _returnvalue_2 _compastimetogrowstart)
      (Transformation|SetWorldScale3D _widgetcompass (Math|Vector|MakeVector 1.0 1.0 1.0))
      (if (Variables|Default|Getflag)
        (goto _label))
      (else
        (Transformation|SetWorldScale3D _widgetcompass (Math|Vector|MakeVector 1.0 _returnvalue_6 _returnvalue_6))))))

(fn CompasColorChangeIni
  (if (== self (Game|GetPlayerCharacter 1))
    (Rendering|Material|SetMaterial (Variables|Default|GetWidgetCompass) 0 "/Game/Materials/M_Compass_01.M_Compass_01")
    (else
      (Rendering|Material|SetMaterial (Variables|Default|GetWidgetCompass) 0 "/Game/Materials/MI_Compass_02.MI_Compass_02"))))

(fn CompasRecolor
  (bind _compasstimetochangecolors (Variables|Default|GetCompassTimeToChangeColors))
  (bind _charactermanager (Variables|Default|GetCharacterManager))
  (bind _returnvalue (Class|CharacterManager|GetRemainingSwitchTime _charactermanager))
  (bind _returnvalue_2 (> _returnvalue _compasstimetochangecolors))
  (if (== self (Game|GetPlayerCharacter 1))
    (bind _returnvalue_3 (UserInterface|CreateWidget "/Game/Interface/UI_Compass.UI_Compass_C"))
    (if _returnvalue_2
      (Appearance|SetBrushfromTexture (Variables|/Game/Interface/UI_Compass.UI_Compass_C|GetImage_0 _returnvalue_3) "/Game/Images/SP_CompassOG_01.SP_CompassOG_01" false)
      (UserInterface|SetWidget (Variables|Default|GetWidgetCompass) _returnvalue_3)
      (else
        (Appearance|SetBrushfromTexture (Variables|/Game/Interface/UI_Compass.UI_Compass_C|GetImage_0 _returnvalue_3) "/Game/Images/SP_CompassOR_01.SP_CompassOR_01" false)
        (UserInterface|SetWidget (Variables|Default|GetWidgetCompass) _returnvalue_3)))
    (else
      (bind _returnvalue_4 (UserInterface|CreateWidget "/Game/Interface/UI_Compass.UI_Compass_C"))
      (if _returnvalue_2
        (Appearance|SetBrushfromTexture (Variables|/Game/Interface/UI_Compass.UI_Compass_C|GetImage_0 _returnvalue_4) "/Game/Images/SP_CompassBG_01.SP_CompassBG_01" false)
        (UserInterface|SetWidget (Variables|Default|GetWidgetCompass) _returnvalue_4)
        (else
          (Appearance|SetBrushfromTexture (Variables|/Game/Interface/UI_Compass.UI_Compass_C|GetImage_0 _returnvalue_4) "/Game/Images/SP_CompassBR_01.SP_CompassBR_01" false)
          (UserInterface|SetWidget (Variables|Default|GetWidgetCompass) _returnvalue_4))))))