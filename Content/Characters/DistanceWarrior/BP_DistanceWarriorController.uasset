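; AI controller for the Distance Warrior character, driving it through a behavior tree.
; On BeginPlay it sets up the Distance Warrior blackboard, stores the controlled pawn's location as StartLocation, then runs the behavior tree.
; A GetPlayers helper returns every Twalien actor in the world, though nothing in this controller calls it.
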(event EventBeginPlay
  (Class|AIController|UseBlackboard "/Game/AI/DistanceWarrior/BB_DistanceWarriorBlackboard.BB_DistanceWarriorBlackboard")
  (AI|Components|Blackboard|SetValueasVector (AI|GetBlackboard self) (Variables|Default|GetStartLocation) (Transformation|GetActorLocation (Pawn|GetControlledPawn)))
  (AI|RunBehaviorTree "/Game/AI/DistanceWarrior/BT_DistanceWarriorBehaviour.BT_DistanceWarriorBehaviour"))

(event EventTick
  (params (DeltaSeconds :type Float%20%28single-precision%29)))

(fn ConstructionScript)

(fn GetPlayers
  (bind _outactors (Actor|GetAllActorsOfClass "/Script/Twaliens.Twalien"))
  (return _outactors))