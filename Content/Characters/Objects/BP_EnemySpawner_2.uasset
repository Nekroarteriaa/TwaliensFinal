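; Enemy spawner that keeps one warrior active at a time and destroys itself after two kills.
; On BeginPlay it pauses the CharacterManager's switch timer and records its switch state.
; Tick spawns an enemy, alerts its BasicWarriorController to players in sight, and polls for its death, clearing the alert before self-destruction.
; Helper functions expose the kill count and restart or re-pause the switch timer based on kills and switch state.
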(event EventBeginPlay
  (bind _outactors (Actor|GetAllActorsOfClass "/Script/Twaliens.CharacterManager"))
  (for _array_element _outactors
    (bind _output_get (Variables|Default|SetCaharacterMgr _array_element))
    (bind _returnvalue (Class|CharacterManager|GetSwitchTimerHandle _output_get))
    (Utilities|Time|PauseTimerbyHandle _returnvalue)
    (Variables|Default|SetSwitchState (Variables|/Script/Twaliens.CharacterManager|GetShouldSwitch (Variables|Default|GetCaharacterMgr)))))

(event Collision|EventActorBeginOverlap
  (params (OtherActor :type Actor%20Object%20Reference)))

(event EventTick
  (params (DeltaSeconds :type Float%20%28single-precision%29))
  (if (== (Variables|Default|GetEnemiesSpawned) 0)
    (bind _enemies (Class|EnemySpawner|SpawnEnemywithReference))
    (bind _output_get (Variables|Default|SetEnemies _enemies))
    (if (Utilities|IsValid (Utilities|Array|Get(acopy) _output_get))
      (bind _asbp_basic_warrior_0 (Utilities|Casting|CastToBP_BasicWarrior_0 (Utilities|Array|Get(acopy) _output_get))
        (:then
          (bind _asbasic_warrior_controller (Utilities|Casting|CastToBasicWarriorController (Pawn|GetController _asbp_basic_warrior_0))
            (:then
              (Class|BasicWarriorController|AlertPlayersinSight _asbasic_warrior_controller true)
              (Variables|Default|SetController _asbasic_warrior_controller))
            (:CastFailed
              _)))
        (:CastFailed
          _))
      (bind _result (Math|Integer|IncrementInt (Variables|Default|GetEnemiesSpawned))
        (:%20%20
          (Variables|Default|SetEnemiesSpawned _result)
          (if (== (Variables|Default|GetEnemiesKilled) 2) :!label _label
            (if (Utilities|IsValid (Variables|Default|GetController))
              (Class|BasicWarriorController|AlertPlayersinSight (Variables|Default|GetController) false))
            (Actor|DestroyActor)))))
    (else
      (CallFunction|CountKills)
      (goto _label))))

(fn ConstructionScript)

(fn SwitchCall
  (bind _caharactermgr (Variables|Default|GetCaharacterMgr))
  (bind _returnvalue (Class|CharacterManager|GetSwitchTimerHandle _caharactermgr))
  (if (and (Class|KismetSystemLibrary|IsTimerPausedHandle _returnvalue) (== (Variables|Default|GetEnemiesKilled) 2))
    (Utilities|Time|SetTimerbyFunctionName self "Function" 5.0)
    (Class|CharacterManager|SetSwitchTimerHandle _caharactermgr 5.0)))

(fn GetEnemies
  (bind _outactors (Actor|GetAllActorsOfClass "/Script/Twaliens.BasicWarrior"))
  (for _array_element _outactors
    (bind _returnvalue (Class|BasicWarrior|GetIsDead _array_element))
    (if _returnvalue
      _)))

(fn CountKills
  (bind _enemies (Variables|Default|GetEnemies))
  (bind _output (Utilities|Array|Get(acopy) _enemies))
  (if (Utilities|IsValid _output)
    (bind _returnvalue (Class|BasicWarrior|GetIsDead _output))
    (if _returnvalue
      (bind _result (Math|Integer|IncrementInt (Variables|Default|GetEnemiesKilled))
        (:%20%20
          (Variables|Default|SetEnemiesKilled _result)
          (bind _result_2 (Math|Integer|DecrementInt (Variables|Default|GetEnemiesSpawned))
            (:%20%20
              (Variables|Default|SetEnemiesSpawned _result_2)
              (Utilities|Array|Clear (Variables|Default|GetEnemies)))))))))

(fn Function)

(fn GetEnemiesKilled
  (return (Variables|Default|GetEnemiesKilled)))

(fn ValidateSwitch
  (if (>= (Variables|Default|GetEnemiesKilled) 2)
    (bind _value (CallFunction|ValidateSwicthState))
    (if _value
      (bind _returnvalue (Class|CharacterManager|GetSwitchTimerHandle (Variables|Default|GetCaharacterMgr)))
      (Utilities|Time|PauseTimerbyHandle _returnvalue)
      (return true)
      (else
        (return false)))
    (else
      (return true))))

(fn ValidateSwicthState
  (if (Math|Boolean|NotEqual(Boolean) (Variables|Default|GetSwitchState) (Variables|/Script/Twaliens.CharacterManager|GetShouldSwitch (Variables|Default|GetCaharacterMgr)))
    (return true)
    (else
      (return false))))